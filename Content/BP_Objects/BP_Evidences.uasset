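; BP_Evidences is an evidence actor that makes itself and its attach parent known to the game mode for scanning.
; On BeginPlay it adds itself to BP_GameMode's EvidencesForScan and its parent BP_Object to ActorswEv, both without duplicates.
; It then hides itself in game, and a leftover SetVisibility node is never executed.
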(event EventBeginPlay
  (bind _returnvalue (Game|GetGameMode))
  (bind _self self)
  (bind _asbp_game_mode (Utilities|Casting|CastToBP_GameMode _returnvalue))
  (Utilities|Array|AddUnique (Variables|/Game/BP_GameMode.BP_GameMode_C|GetEvidencesForScan _asbp_game_mode) _self)
  (Utilities|Array|AddUnique (Variables|/Game/BP_GameMode.BP_GameMode_C|GetActorswEv _asbp_game_mode) (.AsBP%20Object (Utilities|Casting|CastToBP_Object (Actor|GetAttachParentActor _self))))
  (if true
    (Rendering|SetActorHiddenInGame self true)))

(fn ConstructionScript)