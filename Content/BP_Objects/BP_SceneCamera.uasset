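; BP_SceneCamera is an interactable viewpoint that zooms the player into a scene to examine attached BP_Objects.
; Interact and EndInteract toggle its prompt widget, whose WB_Interaction points back to this actor.
; Clicking blends the view here, enters cinematic mode, adds WB_NewScene, enables attached objects and sets the character's ActiveCamera.
; Back works in two levels: it resets an investigated item to the scene view, otherwise returns to the player and disables the objects.
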(event Custom|OnClick_Event
  (bind _returnvalue (Game|GetPlayerController 0))
  ;[0.1562 0.1562 0.1562] Scene Zoom in
  (Game|Player|SetViewTargetwithBlend _returnvalue self 1.0 "VTBlend_Linear" 0.0 false)
  (bind _returnvalue_2 (UserInterface|CreateWidget "/Game/UI/Widgets/WB_NewScene.WB_NewScene_C" _returnvalue))
  (bind _output_get (Variables|Default|SetWB_NS _returnvalue_2))
  (UserInterface|Viewport|AddtoViewport _output_get 0)
  (Variables|/Game/UI/Widgets/WB_NewScene.WB_NewScene_C|SetParent _output_get self)
  (Class|PlayerController|SetCinematicMode _returnvalue true true true true true)
  (for _array_element (Actor|GetAttachedActors true false)
    (bind _asbp_object (Utilities|Casting|CastToBP_Object _array_element))
    (Default|Interact _asbp_object)
    (Variables|/Game/ThirdPerson/Blueprints/BP_ThirdPersonCharacter.BP_ThirdPersonCharacter_C|SetActiveCamera (.AsBP%20Third%20Person%20Character (Utilities|Casting|CastToBP_ThirdPersonCharacter (Game|GetPlayerCharacter 0))) (Variables|Default|GetCamera))))

(event Custom|OnBack_Event
  (bind _returnvalue (Game|GetPlayerController 0))
  (Utilities|IsValid (Variables|Default|GetInvestigatingObject)
    (:Is%20Valid
      ;[0.1562 0.1562 0.1562] Quit investigation mode
      (bind _asbp_object (Utilities|Casting|CastToBP_Object (Variables|Default|GetInvestigatingObject)))
      (Transformation|SetRelativeLocation (Variables|/Game/BP_Objects/BP_Object.BP_Object_C|GetItem _asbp_object) (Variables|/Game/BP_Objects/BP_Object.BP_Object_C|GetStartLoc _asbp_object) false false)
      (Transformation|SetRelativeRotation (Variables|/Game/BP_Objects/BP_Object.BP_Object_C|GetItem _asbp_object) (Variables|/Game/BP_Objects/BP_Object.BP_Object_C|GetStartRot _asbp_object) false false)
      (Game|Player|SetViewTargetwithBlend _returnvalue self 1.0 "VTBlend_Linear" 0.0 false)
      (Class|PlayerController|SetCinematicMode _returnvalue true true true true true)
      (Variables|Default|SetInvestigatingObject 0)
      (Widget|SetVisibility (Variables|/Game/UI/Widgets/WB_NewScene.WB_NewScene_C|GetHB_IM (Variables|Default|GetWB_NS)) "Hidden"))
    (:Is%20Not%20Valid
      ;[0.1562 0.1562 0.1562] Quit scene mode
      (Game|Player|SetViewTargetwithBlend _returnvalue (Game|GetPlayerCharacter 0) 1.0 "VTBlend_Linear" 0.0 false)
      (Class|PlayerController|SetCinematicMode _returnvalue false true true true true)
      (Widget|RemovefromParent (Variables|Default|GetWB_NS))
      (for _array_element (Actor|GetAttachedActors true false)
        (bind _asbp_object_2 (Utilities|Casting|CastToBP_Object _array_element))
        (Default|EndInteract _asbp_object_2)))))

(event EventBeginPlay
  (bind _aswb_interaction (Utilities|Casting|CastToWB_Interaction (UserInterface|GetWidget (Variables|Default|GetWidget))))
  (Variables|/Game/UI/Widgets/WB_Interaction.WB_Interaction_C|SetParent _aswb_interaction self))

(event EventInteract
  (Rendering|SetVisibility (Variables|Default|GetWidget) true false))

(event EventEndInteract
  (Rendering|SetVisibility (Variables|Default|GetWidget) false false))

(fn ConstructionScript)

(fn InvestigationMode
  (Transformation|SetActorRelativeLocation (Variables|Default|GetInvestigatingObject) (Variables|/Script/Engine.SceneComponent|GetRelativeLocation (Variables|Default|GetChildActor))))