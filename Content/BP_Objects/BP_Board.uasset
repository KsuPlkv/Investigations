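; BP_Board is an interactable board that switches the player from third-person play to a board view with a WB_NewScene screen.
; On BeginPlay it links itself to its WB_Interaction widget and the player character; Interact and EndInteract show and hide that widget.
; OnClick_Event blends the camera to the board, locks movement and turning through cinematic mode, and adds WB_NewScene to the viewport.
; OnBack_Event returns camera and control and removes the screen.
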(event Custom|OnClick_Event
  (bind _returnvalue (Game|GetPlayerController 0))
  (Game|Player|SetViewTargetwithBlend _returnvalue self 1.0 "VTBlend_Linear" 0.0 false)
  (Class|PlayerController|SetCinematicMode _returnvalue true true true true true)
  (bind _returnvalue_2 (UserInterface|CreateWidget "/Game/UI/Widgets/WB_NewScene.WB_NewScene_C" (Game|GetPlayerController 0) self))
  (bind _output_get (Variables|Default|SetWB_NS _returnvalue_2))
  (UserInterface|Viewport|AddtoViewport _output_get 0))

(event Custom|OnBack_Event
  (bind _returnvalue (Game|GetPlayerController 0))
  (Game|Player|SetViewTargetwithBlend _returnvalue (Game|GetPlayerCharacter 0) 1.0 "VTBlend_Linear" 0.0 false)
  (Class|PlayerController|SetCinematicMode _returnvalue false true true true true)
  (Widget|RemovefromParent (Variables|Default|GetWB_NS)))

(event EventBeginPlay
  (bind _self self)
  (bind _aswb_interaction (Utilities|Casting|CastToWB_Interaction (UserInterface|GetWidget (Variables|Default|GetWidgetInteraction))))
  (Variables|/Game/UI/Widgets/WB_Interaction.WB_Interaction_C|SetParent _aswb_interaction _self)
  (Variables|/Game/ThirdPerson/Blueprints/BP_ThirdPersonCharacter.BP_ThirdPersonCharacter_C|SetBP_Board (.AsBP%20Third%20Person%20Character (Utilities|Casting|CastToBP_ThirdPersonCharacter (Game|GetPlayerCharacter 0))) _self))

(event EventInteract
  (Rendering|SetVisibility (Variables|Default|GetWidgetInteraction) true false))

(event EventEndInteract
  (Rendering|SetVisibility (Variables|Default|GetWidgetInteraction) false false))

(fn ConstructionScript)