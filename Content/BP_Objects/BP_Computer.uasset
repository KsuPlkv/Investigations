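; Interactable computer actor that switches the player from the character view to its own view and opens the WB_NewScene screen.
; On BeginPlay it registers with BP_GameMode, links its Interaction widget to itself and enables mouse-over events.
; Interact and EndInteract show and hide that widget.
; The click event blends the camera in, enters cinematic mode and creates the screen; the back event reverses this.
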(event Custom|OnClick_Event
  (bind _returnvalue (Game|GetPlayerController 0))
  (Game|Player|SetViewTargetwithBlend _returnvalue self 1.0 "VTBlend_Linear" 0.0 false)
  (Class|PlayerController|SetCinematicMode _returnvalue true true true true true)
  (bind _returnvalue_2 (UserInterface|CreateWidget "/Game/UI/Widgets/WB_NewScene.WB_NewScene_C" _returnvalue self))
  (bind _output_get (Variables|Default|SetWB_NS _returnvalue_2))
  (UserInterface|Viewport|AddtoViewport _output_get 0))

(event Custom|OnBack_Event
  (bind _returnvalue (Game|GetPlayerController 0))
  (Game|Player|SetViewTargetwithBlend _returnvalue (Game|GetPlayerCharacter 0) 1.0 "VTBlend_Linear" 0.0 false)
  (Class|PlayerController|SetCinematicMode _returnvalue false true true true true)
  (Widget|RemovefromParent (Variables|Default|GetWB_NS)))

(event EventBeginPlay
  (bind _asbp_game_mode (Utilities|Casting|CastToBP_GameMode (Game|GetGameMode)))
  (Variables|/Game/BP_GameMode.BP_GameMode_C|SetComputer _asbp_game_mode self)
  (bind _aswb_interaction (Utilities|Casting|CastToWB_Interaction (UserInterface|GetWidget (Variables|Default|GetInteraction))))
  (Variables|/Game/UI/Widgets/WB_Interaction.WB_Interaction_C|SetParent _aswb_interaction self)
  (Variables|/Script/Engine.PlayerController|SetbEnableMouseOverEvents (Game|GetPlayerController 0) true))

(event EventInteract
  (Rendering|SetVisibility (Variables|Default|GetInteraction) true false))

(event EventEndInteract
  (Rendering|SetVisibility (Variables|Default|GetInteraction) false false))

(fn ConstructionScript)