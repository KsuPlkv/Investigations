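; BP_Scanner is a scanner actor that sweeps a decal downward and then reveals evidence in the level.
; On BeginPlay it registers itself with BP_GameMode as BPScaner.
; The Scanning event unhides it and steps the decal down on a short delay loop until it reaches zero world height.
; It then hides and resets the decal, unhides the GameMode's EvidencesForScan actors and calls ShowScaned on its ActorswEv.
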(event Custom|Scanning
  (bind _returnvalue (Game|GetGameMode))
  (bind _decal (Variables|Default|GetDecal))
  (bind _returnvalue_2 (Transformation|GetWorldLocation _decal))
  (bind _asbp_game_mode (Utilities|Casting|CastToBP_GameMode _returnvalue))
  (Rendering|SetActorHiddenInGame self false)
  (Variables|Default|SetStartLoc (Transformation|GetWorldLocation _decal))
  (if (> (.z _returnvalue_2) 0.0) :!label _label
    (Transformation|SetWorldLocation _decal (Math|Vector|MakeVector (.x _returnvalue_2) (.y _returnvalue_2) (- (.z _returnvalue_2) 11.0)) false false)
    (Utilities|FlowControl|Delay 0.1)
    (goto _label)
    (else
      (Rendering|SetActorHiddenInGame self true)
      (Transformation|SetWorldLocation (Variables|Default|GetDecal) (Variables|Default|GetStartLoc) false false)
      (for _array_element (Variables|/Game/BP_GameMode.BP_GameMode_C|GetEvidencesForScan _asbp_game_mode)
        (Rendering|SetActorHiddenInGame _array_element false))
      (for _array_element_2 (Variables|/Game/BP_GameMode.BP_GameMode_C|GetActorswEv _asbp_game_mode)
        (Default|ShowScaned _array_element_2)))))

(event EventBeginPlay
  (Variables|/Game/BP_GameMode.BP_GameMode_C|SetBP_Scaner (.AsBP%20Game%20Mode (Utilities|Casting|CastToBP_GameMode (Game|GetGameMode))) self))

(fn ConstructionScript)