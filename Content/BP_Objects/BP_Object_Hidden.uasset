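; BP_Object_Hidden is an investigable evidence object, optionally hidden at start, that shows an interaction widget.
; Clicking enters investigation mode, via the parent scene camera or its own view blend and WB_NewScene, and logs a note.
; Input axes rotate the item.
; IMPowder stamps brush textures into a render target feeding the item's dynamic material, allowing powder to be painted on it.
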(event Custom|OnClick_Event
  (bind _returnvalue (Actor|GetAttachParentActor))
  (bind _returnvalue_2 (Game|GetPlayerController 0))
  (bind _item (Variables|Default|GetItem))
  (bind _asbp_scene_camera (Utilities|Casting|CastToBP_SceneCamera _returnvalue))
  (if (.isinscene (Variables|Default|GetStructure))
    (Variables|/Game/BP_Objects/BP_SceneCamera.BP_SceneCamera_C|SetInvestigatingObject _asbp_scene_camera self)
    (Default|InvModeBegin (Variables|/Game/BP_Objects/BP_SceneCamera.BP_SceneCamera_C|GetWB_NS _asbp_scene_camera))
    (Default|InvestigationMode _asbp_scene_camera)
    (else
      (Game|Player|SetViewTargetwithBlend _returnvalue_2 self 1.0 "VTBlend_Linear" 0.0 false)
      (Class|PlayerController|SetCinematicMode _returnvalue_2 true true true true true)
      (bind _returnvalue_3 (UserInterface|CreateWidget "/Game/UI/Widgets/WB_NewScene.WB_NewScene_C" 0 0))
      (UserInterface|Viewport|AddtoViewport _returnvalue_3 0)
      (Default|InvModeBegin _returnvalue_3 self)
      (CallFunction|InvestigationMode)))
  (Variables|Default|SetStartLoc (Variables|/Script/Engine.SceneComponent|GetRelativeLocation _item))
  (Variables|Default|SetStartRot (Variables|/Script/Engine.SceneComponent|GetRelativeRotation _item))
  (Input|EnableInput (Game|GetPlayerController 0))
  ;[0.8177 0.4441 0.08944] Brushing
  (bind _returnvalue_4 (Rendering|CreateRenderTarget2D 512 512 "RTF_RGBA16f"))
  (bind _output_get (Variables|Default|SetRT _returnvalue_4))
  (bind _returnvalue_5 (Rendering|Material|CreateDynamicMaterialInstance "/Game/3D/vidro.vidro" "None" "None" :!class /Script/Engine.KismetMaterialLibrary))
  (bind _output_get_2 (Variables|Default|SetMCanvas _returnvalue_5))
  (Rendering|Material|SetTextureParameterValue _output_get_2 "RenT" (Variables|Default|GetRT))
  (Rendering|Material|SetMaterial (Variables|Default|GetItem) 0 _returnvalue_5)
  (bind _returnvalue_6 (Rendering|Material|CreateDynamicMaterialInstance "/Game/Materials/M_Powder.M_Powder" "None" "None" :!class /Script/Engine.KismetMaterialLibrary))
  (Variables|Default|SetPowderM _returnvalue_6)
  (CallFunction|BLAddNote (Variables|Default|GetStructure)))

(event EventBeginPlay
  (bind _aswb_interaction (Utilities|Casting|CastToWB_Interaction (UserInterface|GetWidget (Variables|Default|GetWidget))))
  (Variables|/Game/UI/Widgets/WB_Interaction.WB_Interaction_C|SetParent _aswb_interaction self)
  (Variables|/Script/Engine.PlayerController|SetbEnableMouseOverEvents (Game|GetPlayerController 0) true)
  (if (.ishidden (Variables|Default|GetStructure))
    (Rendering|SetActorHiddenInGame self true)))

(event EventInteract
  (Rendering|SetVisibility (Variables|Default|GetWidget) true false))

(event EventEndInteract
  (Rendering|SetVisibility (Variables|Default|GetWidget) false false))

(event Input|AxisEvents|InputAxisInvestigationX
  (params (AxisValue :type Float%20%28single-precision%29))
  (bind _returnvalue (* AxisValue 2.0))
  (bind _item (Variables|Default|GetItem))
  ;[0.1562 0.1562 0.1562] Rotation Input
  (Transformation|SetRelativeRotation _item (Math|Rotator|CombineRotators (Variables|/Script/Engine.SceneComponent|GetRelativeRotation _item) (Math|Rotator|MakeRotator _returnvalue _returnvalue 0.0)) false false))

(event Input|AxisEvents|InputAxisInvestigationY
  (params (AxisValue :type Float%20%28single-precision%29))
  (bind _item (Variables|Default|GetItem))
  ;[0.1562 0.1562 0.1562] Rotation Input
  (Transformation|SetRelativeRotation _item (Math|Rotator|CombineRotators (Variables|/Script/Engine.SceneComponent|GetRelativeRotation _item) (Math|Rotator|MakeRotator 0.0 0.0 (* AxisValue 2.0))) false false))

(event Input|KeyboardEvents|Z
  (params (Key :type Key%20Structure)))

(event Input|KeyboardEvents|X
  (params (Key :type Key%20Structure)))

(fn ConstructionScript)

(fn IMPowder
  (params (LocToPowder :type Vector%202D%20Structure) (Size :type Float%20%28double-precision%29) (Texture :type Texture%202D%20Object%20Reference))
  (bind _returnvalue (/ Size 2.0))
  (bind _powderm (Variables|Default|GetPowderM))
  (Rendering|Material|SetTextureParameterValue _powderm "BrushT" Texture)
  (bind (_canvas _size _context) (Rendering|BeginDrawCanvastoRenderTarget (Variables|Default|GetRT)))
  (Canvas|DrawMaterial :self _canvas :RenderMaterial _powderm :ScreenPosition (- (* _size LocToPowder) _returnvalue) :ScreenSize (Math|Vector2D|MakeVector2D _returnvalue _returnvalue) :CoordinateSize "(X=1.000000,Y=1.000000)" :PivotPoint "(X=0.500000,Y=0.500000)")
  (Rendering|EndDrawCanvastoRenderTarget _context))

(fn InvestigationMode
  (Transformation|SetActorRelativeLocation (Variables|/Script/Engine.SceneComponent|GetRelativeLocation (Variables|Default|GetChildActor))))