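; BP_Scaner is a scanner actor that shows a descending decal sweep when its Scanning event is called.
; On BeginPlay it registers itself as BPScaner on BP_GameMode.
; Scanning unhides the actor and lowers the decal in timed steps through a Delay loop until it reaches world Z zero.
; It then hides the actor and returns the decal to its starting location.
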(event Custom|Scanning
  (bind _decal (Variables|Default|GetDecal))
  (bind _returnvalue (Transformation|GetWorldLocation _decal))
  (Rendering|SetActorHiddenInGame self false)
  (Variables|Default|SetStartLoc (Transformation|GetWorldLocation _decal))
  (if (> (.z _returnvalue) 0.0) :!label _label
    (Transformation|SetWorldLocation _decal (Math|Vector|MakeVector (.x _returnvalue) (.y _returnvalue) (- (.z _returnvalue) 11.0)) false false)
    (Utilities|FlowControl|Delay 0.1)
    (goto _label)
    (else
      (Rendering|SetActorHiddenInGame self true)
      (Transformation|SetWorldLocation (Variables|Default|GetDecal) (Variables|Default|GetStartLoc) false false))))

(event EventBeginPlay
  (Variables|/Game/BP_GameMode.BP_GameMode_C|SetBP_Scaner (.AsBP%20Game%20Mode (Utilities|Casting|CastToBP_GameMode (Game|GetGameMode))) self))

(fn ConstructionScript)