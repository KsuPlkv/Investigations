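; BP_Marker is a marker actor with a number widget that re-orients when the camera changes.
; On BeginPlay it sets the widget to a default tilt and adds itself to the MarkersArray in BP_GameMode.
; OnChangeCamera_Event adds the given angle to the widget's yaw, or restores the default rotation when the angle is zero.
; Both branches print debug strings.
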(event Custom|OnChangeCamera_Event
  (params (Angle :type Integer))
  (bind _numberwidget (Variables|Default|GetNumberWidget))
  (bind _relativerotation (Variables|/Script/Engine.SceneComponent|GetRelativeRotation _numberwidget))
  (if (== Angle 0)
    (Transformation|SetRelativeRotation _numberwidget "40.000000,0.000000,0.000000" false false)
    (Development|PrintString "bye")
    (else
      (Transformation|SetRelativeRotation _numberwidget (Math|Rotator|MakeRotator (.roll _relativerotation) (.pitch _relativerotation) (+ (.yaw _relativerotation) Angle)) false false)
      (Development|PrintString "Hello"))))

(event EventBeginPlay
  (Transformation|SetRelativeRotation (Variables|Default|GetNumberWidget) "40.000000,0.000000,0.000000" false false)
  (Utilities|Array|AddUnique (Variables|/Game/BP_GameMode.BP_GameMode_C|GetMarkersArray (.AsBP%20Game%20Mode (Utilities|Casting|CastToBP_GameMode (Game|GetGameMode)))) self))

(fn ConstructionScript)